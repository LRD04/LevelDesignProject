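; Hinged door Blueprint that swings open when the player character enters its box trigger, requiring a collected key if locked.
; With CollectedKey set on the first BP_ThirdPersonCharacter found, it clears IsLocked and plays a Timeline lerping the Scene component's rotation.
; Unlocked doors just play the Timeline, and nothing closes them.
; Key removal on finish requires IsLocked, already cleared by then, so the key stays.
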(event `self.BoxCollision.OnComponentBeginOverlap`
  (params (OverlappedComponent :type "PrimitiveComponent Object Reference") (OtherActor :type "Actor Object Reference") (OtherComp :type "PrimitiveComponent Object Reference") (OtherBodyIndex :type Integer) (bFromSweep :type Boolean) (SweepResult :type "HitResult Structure (by ref)"))
  ;[1 1 1] Event: Overlap
  ;[1 1 1] Checks if it is Player Character + If Key Collected
  (if (== OtherActor (`GameplayStatics.GetPlayerCharacter` 0))
    (if (`self.IsLocked?`)
      (bind _outactors (`GameplayStatics.GetAllActorsOfClass` "/Game/ThirdPerson/Blueprints/BP_ThirdPersonCharacter.BP_ThirdPersonCharacter_C"))
      (bind _output (`|GetArrayItem` _outactors))
      (if (`/Game/ThirdPerson/Blueprints/BP_ThirdPersonCharacter.CollectedKey` _output)
        (set `self.IsLocked?` false)
        ;[1 1 1] Timeline: Outputs a Value every frame
        (bind (_direction _newtrack_0) (`Timeline|Timeline` :!label _label)
          (:`Update`
            ;[1 1 1] Tells the component what to move (rotation or  location).
            (`SceneComponent.K2_SetRelativeRotation` (`self.Scene`) (`KismetMathLibrary.RLerp` (`self.DoorBeginRotation`) (`self.DoorEndRotation`) _newtrack_0) false false))
          (:`Finished`
            ;[1 1 1] Remove Key
            (bind _outactors_2 (`GameplayStatics.GetAllActorsOfClass` "/Game/ThirdPerson/Blueprints/BP_ThirdPersonCharacter.BP_ThirdPersonCharacter_C"))
            (if (`self.IsLocked?`)
              (if (`/Game/ThirdPerson/Blueprints/BP_ThirdPersonCharacter.CollectedKey` (`|GetArrayItem` _outactors_2))
                (set `/Game/ThirdPerson/Blueprints/BP_ThirdPersonCharacter.CollectedKey` false _output))))))
      (else
        (goto _label)))))

(fn `UserConstructionScript`)